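; Controller Blueprint for a widget-driven UI with a rocket simulation, which on BeginPlay sets UI-only input with a visible cursor and caches the master and simulator widgets.
; Timelines track button hold time and a restartable, self-looping Milliseconds clock.
; Next/Previous functions cycle a wrapping widget ID, while input toggles by adding an empty viewport widget or removing all widgets.
; RocketCheckFinalResult is an empty stub with disconnected pass/fail logic.
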(event Custom|Resume%20Timeline
  (bind _milliseconds (Timeline|Timeline_0 Play)
    (:Update
      (Variables|Default|SetMilliseconds _milliseconds))
    (:Finished
      (CallFunction|RestartTimeline))))

(event Custom|Pause%20Timeline
  (bind _milliseconds (Timeline|Timeline_0 Stop)
    (:Update
      (Variables|Default|SetMilliseconds _milliseconds))
    (:Finished
      (CallFunction|RestartTimeline))))

(event Custom|Held%20Start
  (bind _newtrack_0 (Timeline|Button%20held%20down Play)
    (:Update
      (Variables|Default|SetTimeHeldDown _newtrack_0))
    (:Finished
      (Variables|Default|SetTimeHeldDown 1.0))))

(event Custom|Restart%20Timeline
  (bind _milliseconds (Timeline|Timeline_0 PlayFromStart)
    (:Update
      (Variables|Default|SetMilliseconds _milliseconds))
    (:Finished
      (CallFunction|RestartTimeline))))

(event Custom|Held%20Stop
  (bind _newtrack_0 (Timeline|Button%20held%20down Stop)
    (:Update
      (Variables|Default|SetTimeHeldDown _newtrack_0))
    (:Finished
      (Variables|Default|SetTimeHeldDown 1.0))))

(event Custom|Restar%20Held
  (bind _newtrack_0 (Timeline|Button%20held%20down PlayFromStart)
    (:Update
      (Variables|Default|SetTimeHeldDown _newtrack_0))
    (:Finished
      (Variables|Default|SetTimeHeldDown 1.0))))

(event EventBeginPlay
  (bind _returnvalue (Game|GetPlayerController 0))
  (Input|SetInputModeUIOnly _returnvalue 0 "LockInFullscreen")
  (Variables|/Script/Engine.PlayerController|SetbShowMouseCursor _returnvalue true)
  (bind _foundwidgets (Widget|GetAllWidgetsOfClass "/Game/Widgets/WPP_Master.WPP_Master_C" false))
  (Variables|Default|SetMaster (Utilities|Array|Get(acopy) _foundwidgets))
  (bind _foundwidgets_2 (Widget|GetAllWidgetsOfClass "/Game/Widgets/RocketBuilding/WBP_RocketSimulation.WBP_RocketSimulation_C" false))
  (Variables|Default|SetSimulatorWidget (Utilities|Array|Get(acopy) _foundwidgets_2)))

(event Collision|EventActorBeginOverlap
  (params (OtherActor :type Actor%20Object%20Reference)))

(event EventTick
  (params (DeltaSeconds :type Float%20%28single-precision%29)))

(event Input|ActionEvents|InputActionNext
  (params (Key :type Key%20Structure :default "None")))

(fn ConstructionScript)

(fn DesactivateInput
  (bind _returnvalue (UserInterface|CreateWidget "/Game/Widgets/Minigames/WPS_Empty.WPS_Empty_C"))
  (UserInterface|Viewport|AddtoViewport _returnvalue 0)
  (Development|PrintString "InputDisactivated"))

(fn ActivateInput
  (Viewport|RemoveAllWidgets))

(fn RocketCheckFinalResult)

(fn NextWidget
  (bind _output_get (Variables|Default|SetWidgetID%20BP (+ (Variables|Default|GetWidgetID%20BP) 1)))
  (if (> _output_get (Variables|Default|GetNumber%20of%20Widgets))
    (Variables|Default|SetWidgetID%20BP 1)))

(fn PreviousWidget
  (if (> (Variables|Default|GetWidgetID%20BP) 1)
    (Variables|Default|SetWidgetID%20BP (- (Variables|Default|GetWidgetID%20BP) 1))
    (else
      (Variables|Default|SetWidgetID%20BP (Variables|Default|GetNumber%20of%20Widgets)))))

(fn NewFunction0)