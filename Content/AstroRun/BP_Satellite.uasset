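; BP_Satellite is a Paper2D sprite hazard in AstroRun that kills the astronaut on contact.
; Its construction script gives the sprite a random scale per axis and randomly mirrors it on X for visual variety.
; Tick moves the actor along world Y by Speed, scaled by delta time and without sweeping.
; Any overlap with BP_AstroCharacter calls that character's Death function.
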(event EventBeginPlay)

(event Collision|EventActorBeginOverlap
  (params (OtherActor :type Actor%20Object%20Reference))
  (bind _asbp_astro_character (Utilities|Casting|CastToBP_AstroCharacter OtherActor))
  (Default|Death _asbp_astro_character))

(event EventTick
  (params (DeltaSeconds :type Float%20%28single-precision%29))
  (Transformation|AddActorWorldOffset (Math|Vector|MakeVector 0.0 (* DeltaSeconds (Variables|Default|GetSpeed) 1.0) 0.0)))

(fn ConstructionScript
  (bind _returnvalue (Math|Random|RandomFloatinRange 0.25 0.5))
  (bind _returnvalue_2 (Math|Random|RandomFloatinRange 0.25 0.5))
  (switch int (Math|Random|RandomIntegerinRange 0 1)
    (:0
      (Transformation|SetRelativeScale3D (Variables|Default|GetPaperSprite) (Math|Vector|MakeVector (* 1 _returnvalue_2) _returnvalue_2 _returnvalue_2)))
    (:1
      (Transformation|SetRelativeScale3D (Variables|Default|GetPaperSprite) (Math|Vector|MakeVector (* -1 _returnvalue) _returnvalue _returnvalue)))))