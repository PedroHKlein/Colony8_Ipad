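; BP_Asteroid is a moving hazard in AstroRun that calls Death on any BP_AstroCharacter overlapping it.
; Tick moves the actor along world Y at its Speed without sweeping and spins the Paper sprite at a constant pitch rate.
; The construction script varies each asteroid by randomizing the sprite's scale independently per axis and its vertical offset.
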(event EventBeginPlay)

(event Collision|EventActorBeginOverlap
  (params (OtherActor :type Actor%20Object%20Reference))
  (bind _asbp_astro_character (Utilities|Casting|CastToBP_AstroCharacter OtherActor))
  (Default|Death _asbp_astro_character))

(event EventTick
  (params (DeltaSeconds :type Float%20%28single-precision%29))
  (Transformation|AddActorWorldOffset (Math|Vector|MakeVector 0.0 (* DeltaSeconds (Variables|Default|GetSpeed) 1.0) 0.0))
  (Transformation|AddLocalRotation (Variables|Default|GetPaperSprite) (Math|Rotator|MakeRotator 0.0 (* DeltaSeconds 1.8e+02) 0.0) false false))

(fn ConstructionScript
  (bind _returnvalue (Math|Random|RandomFloatinRange 0.25 0.4))
  (Transformation|SetRelativeScale3D (Variables|Default|GetPaperSprite) (Math|Vector|MakeVector _returnvalue _returnvalue _returnvalue))
  (Transformation|SetRelativeLocation (Variables|Default|GetPaperSprite) (Math|Vector|MakeVector 0.0 0.0 (Math|Random|RandomFloatinRange 75.0 1e+01)) false false))