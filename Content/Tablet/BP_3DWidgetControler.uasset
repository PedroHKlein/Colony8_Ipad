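; BP_3DWidgetControler is a controller for the tablet's widget UI and its rocket simulation.
; BeginPlay sets UI-only input with a visible cursor and caches the WPP_Master and WBP_RocketSimulation widgets.
; Next/Previous Widget cycle a wrapping page ID; DesactivateInput overlays WPS_Empty, and ActivateInput removes all widgets.
; RocketCheckFinalResult is an empty stub, with its module-result checks left unconnected.
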(event EventBeginPlay
  (bind _returnvalue (Game|GetPlayerController 0))
  (Input|SetInputModeUIOnly _returnvalue 0 "LockInFullscreen")
  (Variables|/Script/Engine.PlayerController|SetbShowMouseCursor _returnvalue true)
  (bind _foundwidgets (Widget|GetAllWidgetsOfClass "/Game/Tablet/WPP_Master.WPP_Master_C" false))
  (Variables|Default|SetMaster (Utilities|Array|Get(acopy) _foundwidgets))
  (bind _foundwidgets_2 (Widget|GetAllWidgetsOfClass "/Game/Tablet/RocketBuilding/WBP_RocketSimulation.WBP_RocketSimulation_C" false))
  (Variables|Default|SetSimulatorWidget (Utilities|Array|Get(acopy) _foundwidgets_2)))

(event Collision|EventActorBeginOverlap
  (params (OtherActor :type Actor%20Object%20Reference)))

(event EventTick
  (params (DeltaSeconds :type Float%20%28single-precision%29)))

(event Input|ActionEvents|InputActionNext
  (params (Key :type Key%20Structure :default "None")))

(fn ConstructionScript)

(fn DesactivateInput
  (bind _returnvalue (UserInterface|CreateWidget "/Game/Tablet/Minigame/WPS_Empty.WPS_Empty_C"))
  (UserInterface|Viewport|AddtoViewport _returnvalue 0)
  (Development|PrintString "InputDisactivated"))

(fn ActivateInput
  (Viewport|RemoveAllWidgets))

(fn RocketCheckFinalResult)

(fn NextWidget
  (bind _output_get (Variables|Default|SetWidgetID%20BP (+ (Variables|Default|GetWidgetID%20BP) 1)))
  (if (> _output_get (Variables|Default|GetNumber%20of%20Widgets))
    (Variables|Default|SetWidgetID%20BP 1)))

(fn PreviousWidget
  (if (> (Variables|Default|GetWidgetID%20BP) 1)
    (Variables|Default|SetWidgetID%20BP (- (Variables|Default|GetWidgetID%20BP) 1))
    (else
      (Variables|Default|SetWidgetID%20BP (Variables|Default|GetNumber%20of%20Widgets)))))