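; Minigame controller actor that shows the WPS_SliderEnergyBar slider widget on screen.
; BeginPlay and every Menu press (both FlipFlop branches) create and add a new widget, switch to UI-only input and show the cursor, without removing earlier widgets.
; ActivateInput and DesactivateInput toggle cursor and mouse events, the latter also restoring game-only input and disabling the actor's input; neither is called here.
; The viewport-centring logic is disconnected.
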(event EventBeginPlay
  (bind _returnvalue (Game|GetPlayerController 0))
  (bind _returnvalue_2 (UserInterface|CreateWidget "/Game/Minigame/WPS_SliderEnergyBar.WPS_SliderEnergyBar_C" _returnvalue))
  (UserInterface|Viewport|AddtoViewport _returnvalue_2 0)
  (Input|SetInputModeUIOnly _returnvalue _returnvalue_2 "DoNotLock")
  (Variables|/Script/Engine.PlayerController|SetbShowMouseCursor _returnvalue true))

(event Input|ActionEvents|InputActionMenu
  (params (Key :type Key%20Structure))
  (bind _returnvalue (Game|GetPlayerController 0))
  (:Pressed
    (Utilities|FlowControl|FlipFlop
      (:A
        _)
      (:B
        _))
    (bind _returnvalue_2 (UserInterface|CreateWidget "/Game/Minigame/WPS_SliderEnergyBar.WPS_SliderEnergyBar_C" _returnvalue))
    (UserInterface|Viewport|AddtoViewport _returnvalue_2 0)
    (Input|SetInputModeUIOnly _returnvalue _returnvalue_2 "DoNotLock")
    (Variables|/Script/Engine.PlayerController|SetbShowMouseCursor _returnvalue true)))

(fn ConstructionScript)

(fn DesactivateInput
  (bind _returnvalue (Game|GetPlayerController 0))
  (Variables|/Script/Engine.PlayerController|SetbEnableMouseOverEvents _returnvalue false)
  (Variables|/Script/Engine.PlayerController|SetbEnableClickEvents _returnvalue false)
  (Variables|/Script/Engine.PlayerController|SetbShowMouseCursor _returnvalue false)
  (Input|DisableInput _returnvalue)
  (Input|SetInputModeGameOnly _returnvalue))

(fn ActivateInput
  (bind _returnvalue (Game|GetPlayerController 0))
  (Variables|/Script/Engine.PlayerController|SetbEnableMouseOverEvents _returnvalue true)
  (Variables|/Script/Engine.PlayerController|SetbEnableClickEvents _returnvalue true)
  (Variables|/Script/Engine.PlayerController|SetbShowMouseCursor _returnvalue true))